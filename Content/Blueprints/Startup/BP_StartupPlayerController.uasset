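; Startup player controller that chooses between a VR and a desktop character when play begins.
; If IsVRDesired is set and the HMD enables, it spawns the VR character, otherwise falling back to desktop.
; Either pawn spawns at a PlayerStart, is possessed, and gets its own Enhanced Input mapping context with game-only input.
; The VR spawn is lowered and takes only location and scale from the start, not rotation.
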(event `self.ReceiveBeginPlay`
  (if (`self.Is VR Desired?`)
    (bind _returnvalue (`HeadMountedDisplayFunctionLibrary.EnableHMD` true))
    (if _returnvalue
      (`self.Start VR Character`)
      (else
        (`self.Start Desktop Character` :!label _label)))
    (else
      (goto _label))))

(event `Start Desktop Character`
  (bind _returnvalue (`GameplayStatics.GetActorOfClass` "/Script/Engine.PlayerStart"))
  (bind _returnvalue_2 (`|SpawnActorFromClass` "/Game/Blueprints/Player/BP_DesktopCharacter.BP_DesktopCharacter_C" (`self.GetTransform` _returnvalue) "AlwaysSpawn" "MultiplyWithRoot" null null))
  (`self.Possess` _returnvalue_2)
  (message `EnhancedInputSubsystemInterface.AddMappingContext` (pcsubsystem `EnhancedInputLocalPlayerSubsystem` self) "/Game/Input/IMC_Default.IMC_Default" 0 (struct))
  (`WidgetBlueprintLibrary.SetInputMode_GameOnly` self))

(event `Start VR Character`
  (bind _returnvalue (`GameplayStatics.GetActorOfClass` "/Script/Engine.PlayerStart"))
  (bind (_returnvalue_location _returnvalue_rotation _returnvalue_scale) (`KismetMathLibrary.BreakTransform` (`self.GetTransform` _returnvalue)))
  (bind _returnvalue_2 (`|SpawnActorFromClass` "/Game/Blueprints/Player/BP_VRCharacter.BP_VRCharacter_C" (`KismetMathLibrary.MakeTransform` (`KismetMathLibrary.MakeVector` (.x _returnvalue_location) (.y _returnvalue_location) (- (.z _returnvalue_location) 45.0)) (struct) _returnvalue_scale) "AlwaysSpawn" "MultiplyWithRoot" null null))
  (`self.Possess` _returnvalue_2)
  (message `EnhancedInputSubsystemInterface.AddMappingContext` (pcsubsystem `EnhancedInputLocalPlayerSubsystem` self) "/Game/Input/IMC_VR_Default.IMC_VR_Default" 0 (struct))
  (`WidgetBlueprintLibrary.SetInputMode_GameOnly` self))

(fn `UserConstructionScript`)