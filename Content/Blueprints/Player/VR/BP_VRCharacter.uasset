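; VR player character that fits a full-body mesh to the player's height and keeps it under the headset.
; BeginPlay scales the mesh from the stored height, assuming a 180-unit mannequin.
; The calibrate input resets HMD orientation and position, derives height from camera Z plus an offset, and rescales against MeshHeight.
; Each tick places the mesh below the camera, following only its yaw, offset by -90 degrees.
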(event `self.ReceiveBeginPlay`
  (`SceneComponent.K2_SetWorldTransform` (`self.Mesh`) (`KismetMathLibrary.MakeTransform` (0.0 0.0 0.0) (struct) (`KismetMathLibrary.Conv_DoubleToVector` (/ (`self.Player Height`) 180.0))) false false))

(event `self.ReceiveTick`
  (params (DeltaSeconds :type "Float (single-precision)"))
  (`self.Update Mesh Position and Rotation`))

(event `EnhancedInput|/Game/Input/Actions/IA_VR_Calibrate`
  (params (ActionValue :type Boolean) (ElapsedSeconds :type "Float (double-precision)") (TriggeredSeconds :type "Float (double-precision)") (InputAction :type "InputAction Object Reference" :default "/Game/Input/Actions/IA_VR_Calibrate.IA_VR_Calibrate"))
  (:`Triggered`
    (`HeadMountedDisplayFunctionLibrary.ResetOrientationAndPosition` 0.0)
    (set `self.Player Height` (+ (.z (.location (`SceneComponent.K2_GetComponentToWorld` (`self.Camera`)))) (`self.HMD height delta`)))
    (`SceneComponent.SetWorldScale3D` (`self.Mesh`) (`KismetMathLibrary.Conv_DoubleToVector` (`KismetMathLibrary.SafeDivide` (`self.Player Height`) (`self.Mesh Height`))))))

(fn `Update Mesh Position and Rotation`
  (bind _camera (`self.Camera`))
  (bind (_returnvalue_roll _returnvalue_pitch _returnvalue_yaw) (`KismetMathLibrary.BreakRotator` (`SceneComponent.K2_GetComponentRotation` _camera)))
  (bind (_returnvalue_x _returnvalue_y _returnvalue_z) (`KismetMathLibrary.BreakVector` (`SceneComponent.K2_GetComponentLocation` _camera)))
  (`SceneComponent.K2_SetWorldLocationAndRotation` (`self.Mesh`) (`KismetMathLibrary.MakeVector` _returnvalue_x _returnvalue_y (- _returnvalue_z (- (`self.Player Height`) (`self.HMD height delta`)))) (`KismetMathLibrary.MakeRotator` 0.0 0.0 (- _returnvalue_yaw 90.0)) false false))

(fn `UserConstructionScript`)