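; BP_Mirror is a mirror actor that moves a SceneCaptureComponent2D in response to the player's position.
; Each Tick it caches player character 0 if needed, then takes the capsule's world offset from the Plane.
; It negates that offset's Y, raises Z by the capsule half height, and applies it as the capture's relative location.
; No rotation is computed; a look-at node toward the Plane sits unused.
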(event `self.ReceiveBeginPlay`)

(event `self.ReceiveTick`
  (params (DeltaSeconds :type "Float (single-precision)"))
  (`/Engine/EditorBlueprintResources/StandardMacros.IsValid` (`self.Player Character`)
    (:`Is Valid`
      _)
    (:`Is Not Valid`
      (bind _output_get (set `self.Player Character` (`GameplayStatics.GetPlayerCharacter` 0)))
      (`/Engine/EditorBlueprintResources/StandardMacros.IsValid` _output_get
        (:`Is Valid`
          _))))
  (bind _capsulecomponent (`Character.CapsuleComponent` _output_get))
  (bind (_returnvalue_x _returnvalue_y _returnvalue_z) (`KismetMathLibrary.BreakVector` (- (`SceneComponent.K2_GetComponentLocation` _capsulecomponent) (`SceneComponent.K2_GetComponentLocation` (`self.Plane`)))))
  (`SceneComponent.K2_SetRelativeLocationAndRotation` :`self` (`self.SceneCaptureComponent2D`) :`NewLocation` (`KismetMathLibrary.MakeVector` _returnvalue_x (* _returnvalue_y -1.0) (+ _returnvalue_z (`CapsuleComponent.CapsuleHalfHeight` _capsulecomponent)))))

(fn `UserConstructionScript`)